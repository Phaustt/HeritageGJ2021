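; BP_HutteBegin is an interactable for the game's opening sequence, where the player places a held mask before the world map loads.
; Tick watches for the player holding a BP_Mask and, gated by a flag, brightens four point lights in a loop containing a Delay.
; Interacting with the mask moves it to MaskPoint, clears the held object and beginning flag, swaps the player's skeletal mesh, then opens Map_World after a delay.
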(event EventTick
  (params (DeltaSeconds :type Float%20%28single-precision%29))
  (if (and (== (Utilities|GetClass (Variables|/Game/UnrealContent/ThirdPersonBP/Blueprints/ThirdPersonCharacter.ThirdPersonCharacter_C|GetHeldObject (Variables|Default|GetPlayer))) "/Game/Dev/Caleb/Detection/BP_Mask.BP_Mask_C") (Variables|Default|GetHa))
    (for _array_element (Variables|Default|Getarray)
      (Rendering|Components|Light|SetIntensity _array_element 5e+03)
      (Utilities|FlowControl|Delay 2.0))
    (Variables|Default|SetHa false)))

(event EventBeginPlay
  (bind _asthird_person_character (Utilities|Casting|CastToThirdPersonCharacter (Game|GetPlayerCharacter 0)))
  (Variables|Default|SetPlayer _asthird_person_character)
  (Variables|Default|Setarray (Utilities|Array|MakeArray (Variables|Default|GetPointLight) (Variables|Default|GetPointLight1) (Variables|Default|GetPointLight3) (Variables|Default|GetPointLight2))))

(event EventFInteract
  (params (IsHeld :type Boolean))
  (bind _player (Variables|Default|GetPlayer))
  (if (== (Utilities|GetClass (Variables|/Game/UnrealContent/ThirdPersonBP/Blueprints/ThirdPersonCharacter.ThirdPersonCharacter_C|GetHeldObject _player)) "/Game/Dev/Caleb/Detection/BP_Mask.BP_Mask_C")
    (bind _asbp_mask (Utilities|Casting|CastToBP_Mask (Variables|/Game/UnrealContent/ThirdPersonBP/Blueprints/ThirdPersonCharacter.ThirdPersonCharacter_C|GetHeldObject _player)))
    (Variables|/Game/Dev/Caleb/Detection/BP_Object.BP_Object_C|SetObjectStates _asbp_mask "NewEnumerator8")
    (Transformation|SetActorLocation (Variables|/Game/UnrealContent/ThirdPersonBP/Blueprints/ThirdPersonCharacter.ThirdPersonCharacter_C|GetHeldObject _player) (Transformation|GetWorldLocation (Variables|Default|GetMask%20point)) false true)
    (Variables|/Game/UnrealContent/ThirdPersonBP/Blueprints/ThirdPersonCharacter.ThirdPersonCharacter_C|SetHeldObject _player 0)
    (bind _asthird_person_character (Utilities|Casting|CastToThirdPersonCharacter (Game|GetPlayerCharacter 0)))
    (Variables|/Game/UnrealContent/ThirdPersonBP/Blueprints/ThirdPersonCharacter.ThirdPersonCharacter_C|SetBegining _asthird_person_character false)
    (Class|SkinnedMeshComponent|SetSkeletalMesh (Variables|/Script/Engine.Character|GetMesh _asthird_person_character) "/Game/Graph/Mesh/Player/player.player" true)
    (Utilities|FlowControl|Delay 2.0)
    (Game|OpenLevel(byObjectReference) "/Game/Maps/Map_World.Map_World")))

(fn ConstructionScript)