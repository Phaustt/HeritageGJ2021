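; BP_Couteau is an interactable knife that can be buried, dug up, or carried by the player or a robot.
; An object state drives Tick, which hides it when buried, pins it to its holder's hold point without collision, or otherwise snaps it to the ground by downward trace.
; FInteract starts a player QTE when buried and handles pickup and drop.
; Player detection runs every tick unless the player holds it.
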(event EventFInteract
  (params (IsHeld :type Boolean))
  (switch Utilities|FlowControl|Switch|SwitchonEnum_ObjectState (Variables|Default|GetObjectStates)
    (:NewEnumerator0
      (Variables|/Game/UnrealContent/ThirdPersonBP/Blueprints/ThirdPersonCharacter.ThirdPersonCharacter_C|SetHeldObject (Variables|Default|GetPlayer) self)
      (Variables|Default|SetObjectStates "NewEnumerator2"))
    (:NewEnumerator1
      (Default|EQTEStart (Variables|Default|GetPlayer))
      (Variables|Default|SetObjectStates "NewEnumerator4"))
    (:NewEnumerator2
      (if IsHeld
        (Variables|Default|SetObjectStates "NewEnumerator0")
        (Collision|SetCollisionEnabled (Variables|Default|GetKnife) "NoCollision")
        (Collision|SetCollisionEnabled (Variables|Default|GetBox) "NoCollision")
        (Variables|/Game/UnrealContent/ThirdPersonBP/Blueprints/ThirdPersonCharacter.ThirdPersonCharacter_C|SetHeldObject (Variables|Default|GetPlayer) 0)))))

(event EventTick
  (params (DeltaSeconds :type Float%20%28single-precision%29))
  (bind _returnvalue (Transformation|GetActorLocation))
  (if (Utilities|Enum|NotEqual(Enum) (Variables|Default|GetObjectStates) "NewEnumerator2")
    (CallFunction|FDetection self (Game|GetPlayerCharacter 0) (Variables|Default|GetMaxDistance) (Variables|Default|GetOnce)))
  (switch Utilities|FlowControl|Switch|SwitchonEnum_ObjectState (Variables|Default|GetObjectStates)
    (:NewEnumerator0
      (Rendering|SetVisibility (Variables|Default|GetKnife) true false)
      (bind _outhit (Collision|LineTraceByChannel _returnvalue (+ _returnvalue (* (Math|Vector|NegateVector (Math|Vector|GetUpVector (Transformation|GetActorRotation))) 5e+03)) "TraceTypeQuery1" false 0 "None"))
      (Transformation|SetActorLocation (.ImpactPoint (Collision|BreakHitResult _outhit)) false true)
      (if (!= (Utilities|GetClass (.HitActor (Collision|BreakHitResult _outhit))) "/Game/UnrealContent/ThirdPersonBP/Blueprints/ThirdPersonCharacter.ThirdPersonCharacter_C")
        (Collision|SetCollisionEnabled (Variables|Default|GetKnife) "QueryAndPhysics")
        (Collision|SetCollisionEnabled (Variables|Default|GetBox) "QueryAndPhysics")))
    (:NewEnumerator1
      (Rendering|SetVisibility (Variables|Default|GetKnife) false false))
    (:NewEnumerator2
      (Transformation|SetActorLocation (Transformation|GetWorldLocation (Variables|/Game/UnrealContent/ThirdPersonBP/Blueprints/ThirdPersonCharacter.ThirdPersonCharacter_C|GetHeldObjectPos (Variables|Default|GetPlayer))) false true)
      (Collision|SetCollisionEnabled (Variables|Default|GetKnife) "NoCollision")
      (Collision|SetCollisionEnabled (Variables|Default|GetBox) "NoCollision"))
    (:NewEnumerator3
      (Transformation|SetActorLocation (Transformation|GetWorldLocation (Variables|/Game/Dev/Caleb/Robot_AI/BP_Robot.BP_Robot_C|GetHeldObjectPos (Variables|Default|GetRobotHeldBy))) false true)
      (Collision|SetCollisionEnabled (Variables|Default|GetKnife) "NoCollision")
      (Collision|SetCollisionEnabled (Variables|Default|GetBox) "NoCollision")
      (Rendering|SetVisibility (Variables|Default|GetKnife) true false))))

(fn ConstructionScript)