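; BP_Four is an interactable furnace-like station that takes wood, then metal, from the player's held object.
; On interact, it accepts only BP_Wood until Tick sees three entries in Holder and sets CanBeUsed, after which it accepts only BP_Metal.
; Each deposit changes the item's state, clears the player's HeldObject and adds to that material's array.
; Once two metals are stored, interacting only prints a debug string.
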(event EventFInteract
  (params (IsHeld :type Boolean))
  (if (>= (Utilities|Array|Length (Variables|Default|GetHolder2)) 2)
    (Development|PrintString "Yeah")
    (else
      (bind _asthird_person_character (Utilities|Casting|CastToThirdPersonCharacter (Game|GetPlayerCharacter 0)))
      (if (Utilities|IsValid (Variables|/Game/UnrealContent/ThirdPersonBP/Blueprints/ThirdPersonCharacter.ThirdPersonCharacter_C|GetHeldObject _asthird_person_character))
        (if (Variables|Default|GetCanBeUsed)
          (Development|PrintString "metal furyyyyy" true true "(R=0.000000,G=0.660000,B=1.000000,A=1.000000)" 0.0)
          (if (== (Utilities|GetClass (Variables|/Game/UnrealContent/ThirdPersonBP/Blueprints/ThirdPersonCharacter.ThirdPersonCharacter_C|GetHeldObject _asthird_person_character)) "/Game/Dev/Caleb/Detection/BP_Metal.BP_Metal_C")
            (bind _asbp_metal (Utilities|Casting|CastToBP_Metal (Variables|/Game/UnrealContent/ThirdPersonBP/Blueprints/ThirdPersonCharacter.ThirdPersonCharacter_C|GetHeldObject _asthird_person_character)))
            (Variables|/Game/Dev/Caleb/Detection/BP_Object.BP_Object_C|SetObjectStates _asbp_metal "NewEnumerator7")
            (Variables|/Game/UnrealContent/ThirdPersonBP/Blueprints/ThirdPersonCharacter.ThirdPersonCharacter_C|SetHeldObject _asthird_person_character 0)
            (Utilities|Array|Add (Variables|Default|GetHolder2) 0)
            (Transformation|SetActorLocation (Transformation|GetActorLocation) false true))
          (elif (== (Utilities|GetClass (Variables|/Game/UnrealContent/ThirdPersonBP/Blueprints/ThirdPersonCharacter.ThirdPersonCharacter_C|GetHeldObject _asthird_person_character)) "/Game/Dev/Caleb/Detection/BP_Wood.BP_Wood_C")
            (bind _asbp_wood (Utilities|Casting|CastToBP_Wood (Variables|/Game/UnrealContent/ThirdPersonBP/Blueprints/ThirdPersonCharacter.ThirdPersonCharacter_C|GetHeldObject _asthird_person_character)))
            (Variables|/Game/Dev/Caleb/Detection/BP_Object.BP_Object_C|SetObjectStates _asbp_wood "NewEnumerator7")
            (Variables|/Game/UnrealContent/ThirdPersonBP/Blueprints/ThirdPersonCharacter.ThirdPersonCharacter_C|SetHeldObject _asthird_person_character 0)
            (Utilities|Array|Add (Variables|Default|GetHolder) 0)
            (Transformation|SetActorLocation (Transformation|GetActorLocation) false true)))))))

(event EventTick
  (params (DeltaSeconds :type Float%20%28single-precision%29))
  (if (>= (Utilities|Array|Length (Variables|Default|GetHolder)) 3)
    (Variables|Default|SetCanBeUsed true)))

(fn ConstructionScript)