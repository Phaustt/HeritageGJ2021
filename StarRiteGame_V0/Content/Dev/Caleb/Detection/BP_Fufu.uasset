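; BP_Fufu is an interactable object that can be buried, sit loose on the ground, or be carried by the player or a robot.
; Each tick it runs detection unless the player holds it, then a state switch sets visibility and collision, following the holder's HeldObjectPos.
; In the default state it snaps to a downward trace hit, with debug drawing and prints left in.
; Interacting picks it up, drops it, or starts the player's QTE when buried.
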(event EventFInteract
  (params (IsHeld :type Boolean))
  (switch Utilities|FlowControl|Switch|SwitchonEnum_ObjectState (Variables|Default|GetObjectStates)
    (:NewEnumerator0
      (Variables|/Game/UnrealContent/ThirdPersonBP/Blueprints/ThirdPersonCharacter.ThirdPersonCharacter_C|SetHeldObject (Variables|Default|GetPlayer) self)
      (Variables|Default|SetObjectStates "NewEnumerator2"))
    (:NewEnumerator1
      (Default|EQTEStart (Variables|Default|GetPlayer))
      (Variables|Default|SetObjectStates "NewEnumerator4"))
    (:NewEnumerator2
      (if IsHeld
        (Variables|Default|SetObjectStates "NewEnumerator0")
        (Collision|SetCollisionEnabled (Variables|Default|GetFufu) "NoCollision")
        (Collision|SetCollisionEnabled (Variables|Default|GetCapsule) "NoCollision")
        (Variables|/Game/UnrealContent/ThirdPersonBP/Blueprints/ThirdPersonCharacter.ThirdPersonCharacter_C|SetHeldObject (Variables|Default|GetPlayer) 0)))))

(event EventTick
  (params (DeltaSeconds :type Float%20%28single-precision%29))
  (bind _returnvalue (Transformation|GetActorLocation))
  (if (Utilities|Enum|NotEqual(Enum) (Variables|Default|GetObjectStates) "NewEnumerator2")
    (CallFunction|FDetection self (Game|GetPlayerCharacter 0) (Variables|Default|GetMaxDistance) (Variables|Default|GetOnce)))
  (switch Utilities|FlowControl|Switch|SwitchonEnum_ObjectState (Variables|Default|GetObjectStates)
    (:NewEnumerator0
      (Development|PrintString "Default" true true "(R=0.000000,G=0.660000,B=1.000000,A=1.000000)" 0.0)
      (Rendering|SetVisibility (Variables|Default|GetFufu) true false)
      (bind _outhit (Collision|LineTraceByChannel _returnvalue (+ _returnvalue (* (Math|Vector|NegateVector (Math|Vector|GetUpVector (Transformation|GetActorRotation))) 5e+03)) "TraceTypeQuery1" false 0 "Persistent"))
      (Transformation|SetActorLocation (.ImpactPoint (Collision|BreakHitResult _outhit)) false true)
      (if (!= (Utilities|GetClass (.HitActor (Collision|BreakHitResult _outhit))) "/Game/UnrealContent/ThirdPersonBP/Blueprints/ThirdPersonCharacter.ThirdPersonCharacter_C")
        (Collision|SetCollisionEnabled (Variables|Default|GetFufu) "QueryAndPhysics")
        (Collision|SetCollisionEnabled (Variables|Default|GetCapsule) "QueryAndPhysics")))
    (:NewEnumerator1
      (Development|PrintString "Buried" true true "(R=0.000000,G=0.660000,B=1.000000,A=1.000000)" 0.0)
      (Rendering|SetVisibility (Variables|Default|GetFufu) false false))
    (:NewEnumerator2
      (Development|PrintString "HeldPlayer" true true "(R=0.000000,G=0.660000,B=1.000000,A=1.000000)" 0.0)
      (Transformation|SetActorLocation (Transformation|GetWorldLocation (Variables|/Game/UnrealContent/ThirdPersonBP/Blueprints/ThirdPersonCharacter.ThirdPersonCharacter_C|GetHeldObjectPos (Variables|Default|GetPlayer))) false true)
      (Collision|SetCollisionEnabled (Variables|Default|GetFufu) "NoCollision")
      (Collision|SetCollisionEnabled (Variables|Default|GetCapsule) "NoCollision"))
    (:NewEnumerator3
      (Development|PrintString "HELdRobot" true true "(R=0.000000,G=0.660000,B=1.000000,A=1.000000)" 0.0)
      (Transformation|SetActorLocation (Transformation|GetWorldLocation (Variables|/Game/Dev/Caleb/Robot_AI/BP_Robot.BP_Robot_C|GetHeldObjectPos (Variables|Default|GetRobotHeldBy))) false true)
      (Collision|SetCollisionEnabled (Variables|Default|GetFufu) "NoCollision")
      (Collision|SetCollisionEnabled (Variables|Default|GetCapsule) "NoCollision")
      (Rendering|SetVisibility (Variables|Default|GetFufu) true false))))

(fn ConstructionScript)