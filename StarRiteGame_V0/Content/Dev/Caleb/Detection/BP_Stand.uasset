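; BP_Stand is an interactable stand that receives a specific object held by the player.
; On BeginPlay it caches the player's ThirdPersonCharacter.
; FInteract checks the held object's class against the stand's Totem number, accepting BP_Fufu or BP_Couteau.
; A matching object is teleported to the Pos component, has its collision disabled and is cleared from the player's HeldObject.
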(event EventFInteract
  (params (IsHeld :type Boolean))
  (bind _player (Variables|Default|GetPlayer))
  (if (Utilities|IsValid (Variables|/Game/UnrealContent/ThirdPersonBP/Blueprints/ThirdPersonCharacter.ThirdPersonCharacter_C|GetHeldObject (Variables|Default|GetPlayer)))
    (if (== (Variables|Default|GetTotem) 1)
      (if (== (Utilities|GetClass (Variables|/Game/UnrealContent/ThirdPersonBP/Blueprints/ThirdPersonCharacter.ThirdPersonCharacter_C|GetHeldObject (Variables|Default|GetPlayer))) "/Game/Dev/Caleb/Detection/BP_Fufu.BP_Fufu_C")
        (Transformation|SetActorLocation (Variables|/Game/UnrealContent/ThirdPersonBP/Blueprints/ThirdPersonCharacter.ThirdPersonCharacter_C|GetHeldObject _player) (Transformation|GetWorldLocation (Variables|Default|Getpos)) false true :!label _label)
        (Collision|SetActorEnableCollision (Variables|/Game/UnrealContent/ThirdPersonBP/Blueprints/ThirdPersonCharacter.ThirdPersonCharacter_C|GetHeldObject _player) false)
        (Variables|/Game/UnrealContent/ThirdPersonBP/Blueprints/ThirdPersonCharacter.ThirdPersonCharacter_C|SetHeldObject _player 0))
      (elif (== (Variables|Default|GetTotem) 2)
        (if (== (Utilities|GetClass (Variables|/Game/UnrealContent/ThirdPersonBP/Blueprints/ThirdPersonCharacter.ThirdPersonCharacter_C|GetHeldObject (Variables|Default|GetPlayer))) "/Game/Dev/Caleb/Detection/BP_Couteau.BP_Couteau_C")
          (goto _label))))))

(event EventBeginPlay
  (bind _asthird_person_character (Utilities|Casting|CastToThirdPersonCharacter (Game|GetPlayerCharacter 0)))
  (Variables|Default|SetPlayer _asthird_person_character))

(fn ConstructionScript)