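; BP_TextIndiceTrigger is a proximity trigger that shows a configurable text, likely a hint, while the player character stands inside its sphere.
; Overlap begin and end events, filtered to the exact ThirdPersonCharacter class, set the Widget's NewText to the Text variable or clear it.
; The construction script sizes the sphere from the Radius variable.
; A debug "Hello" print fires on each entry.
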(event OnComponentBeginOverlap(Sphere)
  (params (OverlappedComponent :type Primitive%20Component%20Object%20Reference) (OtherActor :type Actor%20Object%20Reference) (OtherComp :type Primitive%20Component%20Object%20Reference) (OtherBodyIndex :type Integer) (bFromSweep :type Boolean) (SweepResult :type Hit%20Result%20Structure%20%28by%20ref%29))
  (if (== (Utilities|GetClass OtherActor) "/Game/UnrealContent/ThirdPersonBP/Blueprints/ThirdPersonCharacter.ThirdPersonCharacter_C")
    (Development|PrintString "Hello")
    (Variables|/Game/Dev/Caleb/WBP_Text.WBP_Text_C|SetNewText (Variables|Default|GetWidget) (Utilities|Text|ToText(String) (Variables|Default|GetText)))))

(event OnComponentEndOverlap(Sphere)
  (params (OverlappedComponent :type Primitive%20Component%20Object%20Reference) (OtherActor :type Actor%20Object%20Reference) (OtherComp :type Primitive%20Component%20Object%20Reference) (OtherBodyIndex :type Integer))
  (if (== (Utilities|GetClass OtherActor) "/Game/UnrealContent/ThirdPersonBP/Blueprints/ThirdPersonCharacter.ThirdPersonCharacter_C")
    (Variables|/Game/Dev/Caleb/WBP_Text.WBP_Text_C|SetNewText (Variables|Default|GetWidget) "")))

(fn ConstructionScript
  (Components|Sphere|SetSphereRadius (Variables|Default|GetSphere) (Variables|Default|Getradius) true))